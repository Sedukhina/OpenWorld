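; BP_Platform is a moving platform actor that travels back and forth between its starting position and EndLocation.
; On BeginPlay it stores its location, then a Timeline's Alpha lerps it toward EndLocation, setting the position without sweep.
; Each time the Timeline finishes, a Reverse flag flips to play it in the opposite direction, so the motion repeats endlessly.
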(event EventBeginPlay
  (Variables|Default|SetStartLocation (Transformation|GetActorLocation))
  (bind _alpha (Timeline|Timeline Play)
    (:Update
      (Transformation|SetActorLocation (Math|Vector|Lerp(Vector) (Variables|Default|GetStartLocation) (Variables|Default|GetEndLocation) _alpha) false false))
    (:Finished
      (bind _output_get (Variables|Default|SetReverse (not (Variables|Default|GetReverse))))
      (if _output_get
        (Timeline|Timeline Reverse)
        (else
          (Timeline|Timeline Play))))))

(fn ConstructionScript)